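; BP_ClownBall is a player-controlled physics ball that rolls around in response to Enhanced Input.
; On BeginPlay it adds the default mapping context to player 0's input subsystem.
; Move input applies forces to the Sphere along forward and right vectors derived from control yaw only, so pushes follow the view direction but stay horizontal.
; Look input feeds controller pitch and yaw.
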(event `self.ReceiveBeginPlay`
  (`EnhancedInputSubsystemInterface.AddMappingContext` (pcsubsystem `EnhancedInputLocalPlayerSubsystem` (`GameplayStatics.GetPlayerController` 0)) "/Game/Input/IMC_Default.IMC_Default" 0 (struct)))

(event `EnhancedInput|/Game/Input/Actions/IA_Look`
  (params (ActionValue :type "Vector2D Structure") (ElapsedSeconds :type "Float (double-precision)") (TriggeredSeconds :type "Float (double-precision)") (InputAction :type "InputAction Object Reference" :default "/Game/Input/Actions/IA_Look.IA_Look"))
  (:`Triggered`
    (`self.AddControllerPitchInput` ActionValue_Y)
    (`self.AddControllerYawInput` ActionValue_X)))

(event `EnhancedInput|/Game/Input/Actions/IA_Move`
  (params (ActionValue :type "Vector2D Structure") (ElapsedSeconds :type "Float (double-precision)") (TriggeredSeconds :type "Float (double-precision)") (InputAction :type "InputAction Object Reference" :default "/Game/Input/Actions/IA_Move.IA_Move"))
  (bind (_returnvalue_roll _returnvalue_pitch _returnvalue_yaw) (`KismetMathLibrary.BreakRotator` (`self.GetControlRotation`)))
  (bind _sphere (`self.Sphere`))
  (bind _returnvalue (`KismetMathLibrary.MakeRotator` 0.0 0.0 _returnvalue_yaw))
  (:`Triggered`
    (`PrimitiveComponent.AddForce` _sphere (* (`KismetMathLibrary.GetForwardVector` _returnvalue) ActionValue_Y 20000.0) "None" false)
    (`PrimitiveComponent.AddForce` _sphere (* (`KismetMathLibrary.GetRightVector` _returnvalue) ActionValue_X 20000.0) "None" false)))

(fn `UserConstructionScript`)